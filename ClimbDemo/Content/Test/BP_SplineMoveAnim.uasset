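; BP_SplineMoveAnim is a triggered actor that moves a People mesh along a spline, likely as a test animation.
; A sphere overlap plays a timeline whose Alpha sets the mesh's position and rotation by spline distance, with a yaw offset.
; The timeline also drives an Opacity material parameter, so the mesh starts transparent on BeginPlay and is hidden when the timeline finishes.
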(event `self.ReceiveBeginPlay`
  (`self.SetOpacity` 0.0))

(event `UpdateSpline`
  (bind _spline (`self.Spline`))
  (bind (_direction _alpha _opacity) (`Timeline|Timeline_0` :!via `PlayFromStart`)
    (:`Update`
      (`self.SetOpacity` _opacity)
      (bind _returnvalue (* _alpha (`SplineComponent.GetSplineLength` (`self.Spline`))))
      (`SceneComponent.K2_SetWorldLocation` (`self.People`) (`SplineComponent.GetLocationAtDistanceAlongSpline` _spline _returnvalue "World") false false)
      (bind (_returnvalue_roll _returnvalue_pitch _returnvalue_yaw) (`KismetMathLibrary.BreakRotator` (`SplineComponent.GetRotationAtDistanceAlongSpline` _spline _returnvalue "World")))
      (`SceneComponent.K2_SetWorldRotation` (`self.People`) (`KismetMathLibrary.MakeRotator` _returnvalue_roll _returnvalue_pitch (- _returnvalue_yaw (`self.Z`))) false false))
    (:`Finished`
      (`SceneComponent.SetVisibility` (`self.People`) false false))))

(event `self.Sphere.OnComponentBeginOverlap`
  (params (OverlappedComponent :type "PrimitiveComponent Object Reference") (OtherActor :type "Actor Object Reference") (OtherComp :type "PrimitiveComponent Object Reference") (OtherBodyIndex :type Integer) (bFromSweep :type Boolean) (SweepResult :type "HitResult Structure (by ref)"))
  (`self.UpdateSpline`))

(fn `SetOpacity`
  (params (opacity :type "Float (double-precision)"))
  (`MeshComponent.SetScalarParameterValueOnMaterials` (`self.People`) "Opacity" opacity))

(fn `UserConstructionScript`)