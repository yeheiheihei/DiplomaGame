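; AI for a climbable giant boss that roams or patrols, then chases and attacks climbing characters it detects or is damaged by.
; A looping timer replaces Tick, updating target distance, aim offset yaw/pitch and state.
; Montage sections drive left/right turns, with timeline-lerped rotation, and random attacks, including a roar that flails a climbing target.
; Socket-to-socket sphere traces deal damage, skipping its own limb cling objects.
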(event `Attack`
  (bind _mesh (`self.Mesh`))
  (bind _curtarget (`self.CurTarget`))
  ;[1 0.8064 0.3944] Play Attack montage that tells when to Trace for enemies
  (if (`self.Turning`)
    _
    (elif (not (`self.Attacking`))
      (set `self.Attacking` true)
      (if (`self.TargetIsClimbing`)
        ;;[1 1 1] This randomizes attacks between all of them or just the Roar that flails all cling targets based on if the current target is climbing or not
        (switch `int` (`KismetMathLibrary.RandomIntegerInRange` 1 3)
          (:`1`
            (`|PlayMontage` _mesh "/Game/Clinging/Animations/Montages/GiantAttack_Montage.GiantAttack_Montage" 1.0 0.0 "7"
              (:`then`
                (message `/Game/Clinging/Blueprints/Interfaces/BI_ClingPawn.FlailActor` _curtarget true))
              (:`OnCompleted`
                (message `/Game/Clinging/Blueprints/Interfaces/BI_ClingPawn.FlailActor` _curtarget false)
                (`self.Reset` :!label _label))))
          (:`2`
            (`|PlayMontage` _mesh "/Game/Clinging/Animations/Montages/GiantAttack_Montage.GiantAttack_Montage" 1.0 0.0 (`KismetStringLibrary.Conv_StringToName` (`KismetStringLibrary.Conv_IntToString` (`KismetMathLibrary.RandomIntegerInRange` 1 6))) :!label _label_2
              (:`OnCompleted`
                (goto _label))))
          (:`3`
            (goto _label_2)))
        (else
          (goto _label_2))))))

(event `State_Attack`
  ;[1 1 1] AI States
  ;;[1 0.8064 0.3944] Attack State
  (set `self.bUseControllerRotationYaw` false)
  (`self.GetAngleToTarget` 30.0
    (:`Do Turn`
      (if (`self.Attacking`)
        _
        (elif (not (`self.Turning`))
          (`self.TurnToTarget`)
          (`self.Attack` :!label _label_3))))
    (:`Dont Turn`
      (goto _label_3))))

(event `State_Chase`
  ;[1 1 1] AI States
  ;;[1 0.8064 0.3944] Chase State
  (set `self.bUseControllerRotationYaw` false)
  (if (not (`self.Attacking`))
    (`self.GetAngleToTarget` 60.0
      (:`Do Turn`
        (if (`self.Attacking`)
          _
          (elif (not (`self.Turning`))
            (`self.TurnToTarget`)
            (`self.Chase` (`self.CurTarget`) 400.0 300.0
              (:`InRange`
                (set `self.State` "NewEnumerator4")))))))))

(event `GiantAttackTraces`
  (params (PrimaryStart :type Name) (PrimaryEnd :type Name) (Radius :type "Float (double-precision)"))
  (bind _mesh (`self.Mesh`))
  ;[1 0.8064 0.3944] Uses the ClingObjectAttack array to trace for things to attack when "Trace" is true
  (bind (_outhits _returnvalue) (`KismetSystemLibrary.SphereTraceMulti` :`Start` (`SceneComponent.GetSocketLocation` _mesh PrimaryStart) :`End` (`SceneComponent.GetSocketLocation` _mesh PrimaryEnd) :`Radius` Radius :`TraceChannel` "TraceTypeQuery5" :`DrawDebugType` "ForOneFrame"))
  (if _returnvalue
    (for _array_element _outhits
      (bind (_bblockinghit _binitialoverlap _time _distance _location _impactpoint _normal _impactnormal _physmat _hitactor) (`GameplayStatics.BreakHitResult` _array_element))
      (bind _asbp_base_cling_object (cast `/Game/Clinging/Blueprints/Components/BP_BaseClingObject` _hitactor)
        (:`then`
          (if (not (`KismetArrayLibrary.Array_Contains` (`self.AllLimbObjects`) _asbp_base_cling_object))
            (`GameplayStatics.ApplyDamage` _hitactor 10.0 null self :!label _label_4)))
        (:`CastFailed`
          (goto _label_4))))))

(event `TurnToTarget`
  (bind (_returnvalue_roll _returnvalue_pitch _returnvalue_yaw) (`KismetMathLibrary.BreakRotator` (`KismetMathLibrary.FindLookAtRotation` (`self.K2_GetActorLocation`) (`self.K2_GetActorLocation` (`self.CurTarget`)))))
  ;[1 0.8064 0.3944] Turn to look at Target
  (if (`self.Attacking`)
    _
    (elif (`self.TargetIsClimbing`)
      _
      (elif (not (`self.Turning`))
        (set `self.Turning` true)
        (`|PlayMontage` (`self.Mesh`) "/Game/Clinging/Animations/Montages/GiantTurn_Montage.GiantTurn_Montage" 1.0 0.0 (`KismetStringLibrary.Conv_StringToName` (`KismetStringLibrary.Conv_IntToString` (`self.TurnNum`)))
          (:`then`
            (bind (_direction _alpha) (`Timeline|Timeline_0` :!via `PlayFromStart` :!label _label_5)
              (:`Update`
                (`self.K2_SetActorRotation` (`KismetMathLibrary.RLerp` (`self.K2_GetActorRotation`) (`KismetMathLibrary.MakeRotator` 0.0 0.0 _returnvalue_yaw) _alpha true))
                (if (`self.TargetIsClimbing`)
                  (goto _label_5 :!via `Stop`)))))
          (:`OnCompleted`
            (`self.Reset`)))))))

(event `State_Patrol`
  ;[1 1 1] AI States
  ;;[1 0.8064 0.3944] Patrol State
  (set `self.bUseControllerRotationYaw` false)
  (if (`self.Turning`)
    _
    (elif (not (`self.Patrolling`))
      (set `self.Patrolling` true)
      (`|AIMoveTo` self (0.0 0.0 0.0) (`|GetArrayItem` (`self.PatrolPoints`) (`self.PatrolPointIndex`))
        (:`OnSuccess`
          (`/Engine/EditorBlueprintResources/StandardMacros.IncrementInt` (`self.PatrolPointIndex`)
            (:`  `
              _)))
        (:`OnFail`
          _))
      (if (== (`self.PatrolPointIndex`) (`KismetArrayLibrary.Array_Length` (`self.PatrolPoints`)))
        (set `self.PatrolPointIndex` 0))
      (`KismetSystemLibrary.Delay` 3.0)
      (`self.GetAngleToPatrolPoint` 60.0
        (:`Do Turn`
          (`self.TurnToPatrolPoint`))
        (:`Dont Turn`
          _))
      (set `self.Patrolling` false))))

(event `State_Roam`
  ;[1 1 1] AI States
  ;;[1 0.8064 0.3944] Roam State
  (`self.GetAngleToPatrolPoint` 60.0
    (:`Do Turn`
      (`self.TurnToPatrolPoint`)
      (if (not (`self.Turning`))
        (if (not (`self.isRoaming`)) :!label _label_6
          (set `self.isRoaming` true)
          (bind _output_get (set `self.RoamLocation` (`NavigationSystemV1.K2_GetRandomLocationInNavigableRadius` (`self.K2_GetActorLocation`) 1000.0 null null))))
        (`|AIMoveTo` self _output_get null 50.0
          (:`OnSuccess`
            (`KismetSystemLibrary.Delay` 3.0)
            (set `self.isRoaming` false)))))
    (:`Dont Turn`
      (goto _label_6))))

(event `self.ReceiveAnyDamage`
  (params (Damage :type "Float (single-precision)") (DamageType :type "DamageType Object Reference") (InstigatedBy :type "Controller Object Reference") (DamageCauser :type "Actor Object Reference"))
  ;[1 1 1] Damaged
  (set `self.Health` (- (`self.Health`) Damage))
  (if (<= (`self.Health`) 0.0)
    (`self.K2_DestroyActor`)
    (else
      (bind _asbp_climbing_character (cast `/Game/Clinging/Blueprints/BP_ClimbingCharacter` DamageCauser))
      (`KismetArrayLibrary.Array_AddUnique` (`self.PotentialTargets`) _asbp_climbing_character)
      (`self.GetRandomTarget`))))

(event `TurnToPatrolPoint`
  (bind (_returnvalue_roll _returnvalue_pitch _returnvalue_yaw) (`KismetMathLibrary.BreakRotator` (`KismetMathLibrary.FindLookAtRotation` (`self.K2_GetActorLocation`) (select `/Game/Clinging/Blueprints/AI/States` (`self.State`) :`NewEnumerator1` (`self.RoamLocation`) :`NewEnumerator5` (`self.K2_GetActorLocation` (`|GetArrayItem` (`self.PatrolPoints`) (`self.PatrolPointIndex`)))))))
  ;[1 0.8064 0.3944] Turn to look at Patrol Point
  (if (`self.Attacking`)
    _
    (elif (not (`self.Turning`))
      (set `self.Turning` true)
      (`|PlayMontage` (`self.Mesh`) "/Game/Clinging/Animations/Montages/GiantTurn_Montage.GiantTurn_Montage" 1.0 0.0 (`KismetStringLibrary.Conv_StringToName` (`KismetStringLibrary.Conv_IntToString` (`self.TurnNum`)))
        (:`then`
          (bind (_direction _alpha) (`Timeline|Timeline_1` :!via `PlayFromStart`)
            (:`Update`
              (`self.K2_SetActorRotation` (`KismetMathLibrary.RLerp` (`self.K2_GetActorRotation`) (`KismetMathLibrary.MakeRotator` 0.0 0.0 _returnvalue_yaw) _alpha true)))))
        (:`OnCompleted`
          (`self.Reset`))))))

(event `Reset`
  ;[1 0.8064 0.3944] Reset variables
  (set `self.Attacking` false)
  (set `self.Turning` false)
  (set `self.Trace` false)
  (`self.GetRandomTarget`))

(event `self.Detection.OnComponentBeginOverlap`
  (params (OverlappedComponent :type "PrimitiveComponent Object Reference") (OtherActor :type "Actor Object Reference") (OtherComp :type "PrimitiveComponent Object Reference") (OtherBodyIndex :type Integer) (bFromSweep :type Boolean) (SweepResult :type "HitResult Structure (by ref)"))
  ;[1 0.8064 0.3944] Detect Enemies
  (bind _asbp_climbing_character (cast `/Game/Clinging/Blueprints/BP_ClimbingCharacter` OtherActor))
  (if (== _asbp_climbing_character (`GameplayStatics.GetPlayerCharacter` 0))
    (set `/Game/Clinging/Blueprints/BP_ClimbingCharacter.Boss` self _asbp_climbing_character))
  (`KismetArrayLibrary.Array_AddUnique` (`self.PotentialTargets`) _asbp_climbing_character)
  (`self.GetRandomTarget`))

(event `self.ReceiveBeginPlay`
  ;[1 0.8064 0.3944] BeginPlay
  ;;[1 1 1] Sets the ClingObjects that can attack in the array
  (for _array_element (`|MakeArray` (`self.Cling_ArmR`) (`self.Cling_ArmL`))
    (`KismetArrayLibrary.Array_AddUnique` (`self.ClingObject_Attack`) _array_element))
  ;;[1 1 1] Puts all Clingobjects In an array
  (for _array_element_2 (`|MakeArray` (`self.Cling_Spine01`) (`self.Cling_ArmL`) (`self.Cling_UpperArmL`) (`self.Cling_ArmR`) (`self.Cling_UpperArmR`) (`self.Cling_Head`) (`self.Cling_Spine03`) (`self.Cling_ThighL`) (`self.Cling_ThighR`) (`self.Cling_CalfL`) (`self.Cling_CalfR`))
    (`KismetArrayLibrary.Array_AddUnique` (`self.AllLimbObjects`) (cast `/Game/Clinging/Blueprints/Components/BP_BaseClingObject` (`ChildActorComponent.ChildActor` _array_element_2) :!pure true)))
  ;;[1 1 1] Puts the mock tick function on a timer to simulate "Event Tick"
  (`KismetSystemLibrary.K2_SetTimer` null "TickFunction" 0.1 true))

(event `TickFunction`
  ;[1 0.8064 0.3944] Function that runs on a timer
  (if (not (`self.Dummy?`))
    (`self.CheckForTarget` 500.0
      (:`Is Valid`
        (`self.CheckIfTargetIsOnSelf`))
      (:`Is Not Valid`
        _))
    (switch `/Game/Clinging/Blueprints/AI/States` (`self.State`)
      (:`NewEnumerator1`
        (`self.State_Roam`))
      (:`NewEnumerator5`
        (`self.State_Patrol`))
      (:`NewEnumerator2`
        (`self.State_Chase`))
      (:`NewEnumerator4`
        (`self.State_Attack`)))))

(event `self.Detection.OnComponentEndOverlap`
  (params (OverlappedComponent :type "PrimitiveComponent Object Reference") (OtherActor :type "Actor Object Reference") (OtherComp :type "PrimitiveComponent Object Reference") (OtherBodyIndex :type Integer))
  (bind _potentialtargets (`self.PotentialTargets`))
  ;[1 0.8064 0.3944] Detect Enemies
  (bind _asbp_climbing_character (cast `/Game/Clinging/Blueprints/BP_ClimbingCharacter` OtherActor))
  (if (== _asbp_climbing_character (`GameplayStatics.GetPlayerCharacter` 0))
    (set `/Game/Clinging/Blueprints/BP_ClimbingCharacter.Boss` null _asbp_climbing_character))
  (if (`KismetArrayLibrary.Array_Contains` _potentialtargets _asbp_climbing_character)
    (`KismetArrayLibrary.Array_RemoveItem` _potentialtargets _asbp_climbing_character)
    (`self.GetRandomTarget`)))

(event `/Game/Clinging/Blueprints/Interfaces/BI_ClingPawn.ModifyClingCharacters`
  (params (`Add?` :type Boolean) (Actor :type "Actor Object Reference"))
  (bind _clingtargets (`self.ClingTargets`))
  (bind _clingtargets_2 (`self.ClingTargets`))
  ;[1 0.8064 0.3944] Interface events
  (if `Add?`
    (if (not (`KismetArrayLibrary.Array_Contains` _clingtargets Actor))
      (`KismetArrayLibrary.Array_AddUnique` _clingtargets Actor))
    (elif (`KismetArrayLibrary.Array_Contains` _clingtargets_2 Actor)
      (`KismetArrayLibrary.Array_RemoveItem` _clingtargets_2 Actor))))

(fn `GetRandomTarget`
  (locals (MaxDistance :type "Float (double-precision)" :default 1000000.0))
  (if (> (`KismetArrayLibrary.Array_Length` (`self.PotentialTargets`)) 0)
    (for _array_element (`self.PotentialTargets`)
      (bind _returnvalue (`self.GetDistanceTo` _array_element))
      (if (< _returnvalue (`local.MaxDistance`))
        (set `local.MaxDistance` _returnvalue)
        (set `self.CurTarget` _array_element)))
    (set `self.State` "NewEnumerator2")
    (else
      (set `self.State` "NewEnumerator1"))))

(fn `UserConstructionScript`)