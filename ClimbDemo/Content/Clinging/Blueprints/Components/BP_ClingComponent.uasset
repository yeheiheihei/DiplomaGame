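; Character component that lets players and AI cling to and climb BP_BaseClingObject actors, including ones on other characters.
; Grab traces attach the character in flying mode, with a hidden spawned cling object as fallback reference.
; While clinging, TickFunction uses sphere traces to align rotation and distance to the surface normal and transfer to adjacent objects.
; It climbs or launches over flat ledges, and lets go on flat surfaces or near ground.
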(event `self.ReceiveTick`
  (params (DeltaSeconds :type "Float (single-precision)")))

(event `JumpUpSurface`
  (bind _character (`self.Character`))
  ;[1 0.8064 0.3944] If surface is flat and we are close enough.. jump up.
  (if (`self.ExitAnimation`)
    (`/Engine/EditorBlueprintResources/StandardMacros.DoOnce` false :!label _label
      (:`Completed`
        (`|PlayMontage` (`Character.Mesh` _character) (`self.ClimbUpAnimation`)
          (:`OnCompleted`
            (`self.LetGoOfEdge` false false 800.0)
            (goto _label :!via `Reset`)))))
    (else
      (`self.LetGoOfEdge` true false 800.0)
      (`KismetSystemLibrary.Delay` 0.5)
      (`Character.LaunchCharacter` (`self.Character`) (* (`Actor.GetActorForwardVector` _character) 500.0) true true))))

(fn `ClingRotation(Climb)`
  (params (`Interpolate?` :type Boolean) (InterpSpeed :type "Float (double-precision)"))
  (locals (LastHitLocation :type "Vector Structure" :default (0.0 0.0 0.0)) (LastHitNormal :type "Vector Structure" :default (0.0 0.0 0.0)))
  (bind _clingobject (`self.ClingObject`))
  (bind _returnvalue (`Actor.K2_GetActorLocation` (`self.Character`)))
  ;[1 1 1] Trace directly to the center of the Clingobject to get the hit location and normal
  (bind (_outhit _returnvalue_2) (`KismetSystemLibrary.SphereTraceSingle` :`Start` _returnvalue :`End` (+ (* (`KismetMathLibrary.GetDirectionUnitVector` _returnvalue (`SceneComponent.K2_GetComponentLocation` (`/Game/Clinging/Blueprints/Components/BP_BaseClingObject.Box` (`self.ClingObject`)))) 150.0) _returnvalue) :`Radius` 10.0 :`TraceChannel` "TraceTypeQuery3" :`TraceColor` (struct :`G` 0.014444 :`B` 0.73791 :`A` 1.0) :`TraceHitColor` (struct :`R` 1.0 :`G` 0.80636 :`B` 0.394398 :`A` 1.0) :`DrawTime` 1.0))
  (if _returnvalue_2
    (bind (_bblockinghit _binitialoverlap _time _distance _location _impactpoint _normal _impactnormal _physmat _hitactor) (`GameplayStatics.BreakHitResult` _outhit))
    (bind (_asbp_base_cling_object _bsuccess) (cast `/Game/Clinging/Blueprints/Components/BP_BaseClingObject` _hitactor :!pure true))
    (if _bsuccess
      (if (== _asbp_base_cling_object (`self.ClingObject`))
        ;[1 1 1] Check if the normal is flat enough to stand oon
        (if (== _normal (0.0 0.0 1.0))
          ;[1 1 1] If the object is on a Character, dont let go
          (if (`/Game/Clinging/Blueprints/Components/BP_BaseClingObject.OnCharacter` (`self.ClingObject`)) :!label _label
            (`self.ChangeLocation` (`local.LastHitLocation`) (`local.LastHitNormal`))
            (return)
            (else
              ;[1 1 1] If we arent on a Character, let go
              (message `/Game/Clinging/Blueprints/Interfaces/ClingAi_BI.ChangeState` (`SkeletalMeshComponent.GetAnimInstance` (`Character.Mesh` (`self.Character`))) "NewEnumerator2")
              (`self.LetGoOfEdge` false)
              (return)))
          (else
            ;[1 1 1] Save the previous location and normal for use
            (set `local.LastHitLocation` _location)
            (set `local.LastHitNormal` _normal)
            (bind _returnvalue_3 (`KismetMathLibrary.FindLookAtRotation` _location (+ _location (* _impactnormal -300.0))))
            ;[1 1 1] Sets Characters rotation
            (`Actor.K2_SetActorRotation` (`self.Character`) (select `bool` `Interpolate?` :`false` _returnvalue_3 :`true` (`KismetMathLibrary.RInterpTo` (`Actor.K2_GetActorRotation` (`self.Character`)) _returnvalue_3 (`GameplayStatics.GetWorldDeltaSeconds`) InterpSpeed)) false)
            ;[1 1 1] Keeps Character From Drifting Away
            (`self.ChangeLocation` (`local.LastHitLocation`) (`local.LastHitNormal`))
            (return)))
        (else
          ;[1 1 1] If the trace hits a different ClingObject than our own, try and attach to it
          (if (`/Game/Clinging/Blueprints/Components/BP_BaseClingObject.CanBeClingedTo` _asbp_base_cling_object)
            (set `/Game/Clinging/Blueprints/Components/BP_BaseClingObject.isBeingClingedTo` true _asbp_base_cling_object)
            (set `/Game/Clinging/Blueprints/Components/BP_BaseClingObject.isBeingClingedTo` false _clingobject)
            (`self.GrabObject` _clingobject _asbp_base_cling_object)
            (else
              (goto _label)))))
      (else
        (goto _label)))
    (else
      (goto _label))))

(fn `GetAdjacentObject`
  (params (MoveForward :type "Float (double-precision)") (MoveRight :type "Float (double-precision)"))
  (bind _character (`self.Character`))
  (bind _clingobject (`self.ClingObject`))
  (bind _returnvalue (`Actor.K2_GetActorLocation` _character))
  (bind _returnvalue_2 (+ _returnvalue (* (`Actor.GetActorForwardVector` _character) 50.0)))
  ;[1 1 1] if we are moving, trace in the direction that we're moving
  (if (== MoveForward 0.0)
    (if (not (== MoveRight 0.0))
      (bind (_outhit _returnvalue_3) (`KismetSystemLibrary.SphereTraceSingle` :`Start` _returnvalue_2 :`End` (+ _returnvalue (* (`PawnMovementComponent.GetLastInputVector` (`Character.CharacterMovement` _character)) 10000.0)) :`Radius` 40.0 :`TraceChannel` "TraceTypeQuery3" :`TraceColor` (struct :`R` 0.149908 :`G` 0.235305 :`B` 1.0 :`A` 1.0) :!label _label))
      (if _returnvalue_3
        (bind (_bblockinghit _binitialoverlap _time _distance _location _impactpoint _normal _impactnormal _physmat _hitactor) (`GameplayStatics.BreakHitResult` _outhit))
        (bind _asbp_base_cling_object (cast `/Game/Clinging/Blueprints/Components/BP_BaseClingObject` _hitactor :!pure true))
        ;[1 1 1] If the trace hits a ClingObject and said ClingObject can be clinged to
        (if (== _asbp_base_cling_object (`self.ClingObject`))
          _
          (elif (`/Game/Clinging/Blueprints/Components/BP_BaseClingObject.CanBeClingedTo` _asbp_base_cling_object)
            (if (< (`KismetMathLibrary.VSize` (- _impactpoint _returnvalue_2)) 150.0)
              ;[1 1 1] Reset old Object and Cling to New ClingObject
              (set `/Game/Clinging/Blueprints/Components/BP_BaseClingObject.isBeingClingedTo` true _asbp_base_cling_object)
              (set `/Game/Clinging/Blueprints/Components/BP_BaseClingObject.isBeingClingedTo` false _clingobject)
              (`self.GrabObject` _clingobject _asbp_base_cling_object)
              (return)
              (else
                _))))))
    (else
      (goto _label)))
  (return))

(fn `GetObjectSurface`
  (bind _clingobject (`self.ClingObject`))
  (bind _character (`self.Character`))
  (bind _returnvalue (`Actor.K2_GetActorRotation` _character))
  (bind _returnvalue_2 (`KismetMathLibrary.GetUpVector` _returnvalue))
  (bind _returnvalue_3 (+ (`Actor.K2_GetActorLocation` _character) (* (`KismetMathLibrary.GetForwardVector` _returnvalue) 75.0)))
  ;[1 1 1] Traces down a little in fornt of the character to get the surface
  (bind (_outhit _returnvalue_4) (`KismetSystemLibrary.SphereTraceSingle` (+ _returnvalue_3 (* _returnvalue_2 200.0)) (+ _returnvalue_3 (* _returnvalue_2 -200.0)) 30.0 "TraceTypeQuery3"))
  (if _returnvalue_4
    (bind (_bblockinghit _binitialoverlap _time _distance _location _impactpoint _normal) (`GameplayStatics.BreakHitResult` _outhit))
    ;[1 1 1] If the surface normal's z is near 1 then it is flat enough to stand on, so climb
    (if (== _normal (0.0 0.0 1.0))
      (if (< (`KismetMathLibrary.VSize` (- _impactpoint (`Actor.K2_GetActorLocation` (`self.Character`)))) 115.0)
        (if (`/Game/Clinging/Blueprints/Components/BP_BaseClingObject.OnCharacter` _clingobject)
          _
          (elif (`/Game/Clinging/Blueprints/Components/BP_BaseClingObject.CanBeClimbed` _clingobject)
            (`self.JumpUpSurface`)
            (return)
            (else
              (`self.LetGoOfEdge` false)
              (return)))))))
  (return))

(fn `GrabObject`
  (params (CurrentObject :type "/Game/Clinging/Blueprints/Components/BP_BaseClingObject Object Reference") (NewObject :type "/Game/Clinging/Blueprints/Components/BP_BaseClingObject Object Reference"))
  (bind _character (`self.Character`))
  (bind _clingobject (`self.ClingObject`))
  (bind _character_2 (`self.Character`))
  (bind _character_3 (`self.Character`))
  (bind _charactermovement (`Character.CharacterMovement` _character_3))
  ;[1 1 1] Attach to the ClingObject and add this Character to the ClingObjects "ClingChars" array
  (`Actor.K2_AttachToActor` _character_2 NewObject "None" "KeepWorld" "KeepWorld" "KeepWorld" true)
  (`PrimitiveComponent.SetCollisionResponseToChannel` (`Character.CapsuleComponent` _character_3) "ECC_GameTraceChannel1" "ECR_Ignore")
  (`CharacterMovementComponent.SetMovementMode` _charactermovement "MOVE_Flying" 0)
  (`MovementComponent.StopMovementImmediately` _charactermovement)
  (set `CharacterMovementComponent.bOrientRotationToMovement` false _charactermovement)
  (set `CharacterMovementComponent.bUseControllerDesiredRotation` false (`Character.CharacterMovement` _character_2))
  (bind _output_get (set `self.ClingObject` NewObject))
  (`/Game/Clinging/Blueprints/Components/BP_BaseClingObject.AddToClingChars` _output_get (`self.Character`))
  (if (`/Game/Clinging/Blueprints/Components/BP_BaseClingObject.ShouldZoomOut?` _clingobject)
    (message `/Game/Clinging/Blueprints/Interfaces/BI_ClingPawn.ChangeCam` _character true)
    (else
      (message `/Game/Clinging/Blueprints/Interfaces/BI_ClingPawn.ChangeCam` _character false)))
  (message `/Game/Clinging/Blueprints/Interfaces/BI_ClingAnimation.Cling?` _character true)
  (set `self.ExitAnimation` (`/Game/Clinging/Blueprints/Components/BP_BaseClingObject.HasExitAnimation` _clingobject))
  (return))

(fn `GrabOn`
  (params (EndPoint :type "Vector Structure"))
  (returns (FoundClingObject :type Boolean))
  (bind _clingobject (`self.ClingObject`))
  ;[1 1 1] Trace to see if we hit a ClingObject, If so, reset variables amd Cling to it
  (bind (_outhit _returnvalue) (`KismetSystemLibrary.SphereTraceSingle` (`Actor.K2_GetActorLocation` (`self.Character`)) EndPoint 30.0 "TraceTypeQuery3"))
  (if _returnvalue
    (bind _asbp_base_cling_object (cast `/Game/Clinging/Blueprints/Components/BP_BaseClingObject` (`.HitActor` (`GameplayStatics.BreakHitResult` _outhit)) :!pure true))
    (if (`/Game/Clinging/Blueprints/Components/BP_BaseClingObject.CanBeClingedTo` _asbp_base_cling_object)
      (`/Engine/EditorBlueprintResources/StandardMacros.IsValid` _clingobject
        (:`Is Valid`
          (set `/Game/Clinging/Blueprints/Components/BP_BaseClingObject.isBeingClingedTo` false _clingobject))
        (:`Is Not Valid`
          _))
      (set `/Game/Clinging/Blueprints/Components/BP_BaseClingObject.isBeingClingedTo` true _asbp_base_cling_object)
      (set `self.isClinging` true)
      (`self.GrabObject` _clingobject _asbp_base_cling_object)
      (return true)
      (else
        _)))
  (return false))

(fn `GrabOn_AI`
  (params (End :type "Vector Structure"))
  (returns (FoundClingObject :type Boolean))
  (bind _clingobject (`self.ClingObject`))
  ;[1 1 1] Trace to see if we hit a ClingObject, If so, reset variables amd Cling to it
  (bind (_outhit _returnvalue) (`KismetSystemLibrary.SphereTraceSingle` (`Actor.K2_GetActorLocation` (`self.Character`)) End 30.0 "TraceTypeQuery3"))
  (if _returnvalue
    (bind (_bblockinghit _binitialoverlap _time _distance _location _impactpoint _normal _impactnormal _physmat _hitactor) (`GameplayStatics.BreakHitResult` _outhit))
    (if (< _distance 300.0)
      (bind _asbp_base_cling_object (cast `/Game/Clinging/Blueprints/Components/BP_BaseClingObject` _hitactor :!pure true))
      (if (`/Game/Clinging/Blueprints/Components/BP_BaseClingObject.CanBeClimbed` _asbp_base_cling_object)
        (`/Engine/EditorBlueprintResources/StandardMacros.IsValid` _clingobject
          (:`Is Valid`
            (set `/Game/Clinging/Blueprints/Components/BP_BaseClingObject.isBeingClingedTo` false _clingobject))
          (:`Is Not Valid`
            _))
        (set `/Game/Clinging/Blueprints/Components/BP_BaseClingObject.isBeingClingedTo` true _asbp_base_cling_object)
        (set `self.isClinging` true)
        (`self.GrabObject` _clingobject _asbp_base_cling_object)
        (return true)
        (else
          _))))
  (return false))

(fn `IsOnGround`
  (bind _character (`self.Character`))
  (bind _returnvalue (`Actor.K2_GetActorLocation` _character))
  ;[1 1 1] Check to see if we are close enough to a flat ground surface that we "should" be able to walk on, then let go
  (bind (_outhit _returnvalue_2) (`KismetSystemLibrary.SphereTraceSingle` _returnvalue (+ _returnvalue (* (`KismetMathLibrary.GetUpVector` (`Actor.K2_GetActorRotation` _character)) -5000.0)) 10.0 "TraceTypeQuery1"))
  (if _returnvalue_2
    (bind (_bblockinghit _binitialoverlap _time _distance _location _impactpoint _normal _impactnormal _physmat _hitactor) (`GameplayStatics.BreakHitResult` _outhit))
    (if (== _impactnormal (0.0 0.0 1.0))
      (if (< (`KismetMathLibrary.VSize` (- _impactpoint (`Actor.K2_GetActorLocation` (`self.Character`)))) 125.0)
        (bind (_asbp_base_cling_object _bsuccess) (cast `/Game/Clinging/Blueprints/Components/BP_BaseClingObject` _hitactor :!pure true))
        (if _bsuccess
          (if (`/Game/Clinging/Blueprints/Components/BP_BaseClingObject.OnCharacter` _asbp_base_cling_object)
            _
            (else
              (`self.LetGoOfEdge` false false 600.0 :!label _label)
              (message `/Game/Clinging/Blueprints/Interfaces/ClingAi_BI.ChangeState` (`self.Character`) "NewEnumerator2")
              (return)))
          (else
            (goto _label))))))
  (return))

(fn `LetGoOfEdge`
  (params (LaunchOnExit :type Boolean) (KeepVelocity :type Boolean) (LaunchVelocity :type "Float (double-precision)"))
  (bind _launchvelocity (`self.LaunchVelocity`))
  (bind _character (`self.Character`))
  (bind _character_2 (`self.Character`))
  (bind _clingobject (`self.ClingObject`))
  (bind _character_3 (`self.Character`))
  (bind _charactermovement (`Character.CharacterMovement` (`self.Character`)))
  ;[1 1 1] Detach Character, reset variables to original, and removes Character from the ClingObjects "ClingChars" array
  (set `self.LaunchVelocity` LaunchVelocity)
  (`Actor.K2_DetachFromActor` _character_2 "KeepWorld" "KeepWorld" "KeepWorld")
  (`PrimitiveComponent.SetCollisionResponseToChannel` (`Character.CapsuleComponent` _character_2) "ECC_GameTraceChannel1" "ECR_Block")
  (`CharacterMovementComponent.SetMovementMode` (`Character.CharacterMovement` _character) "MOVE_Walking" 0)
  (set `/Game/Clinging/Blueprints/Components/BP_BaseClingObject.isBeingClingedTo` false _clingobject)
  (`/Game/Clinging/Blueprints/Components/BP_BaseClingObject.RemoveFromClingChars` _clingobject _character)
  (message `/Game/Clinging/Blueprints/Interfaces/BI_ClingPawn.ChangeCam` (`self.Character`) false)
  (set `self.ClingObject` (`self.OriginalObject`))
  ;[0.3638 0.5792 1] Tells the animBP to stop climbing blendspace
  (message `/Game/Clinging/Blueprints/Interfaces/BI_ClingAnimation.Cling?` (`self.Character`) false)
  ;[1 1 1] Reset Characters movement mode and Rotation
  (set `CharacterMovementComponent.bOrientRotationToMovement` true _charactermovement)
  (set `CharacterMovementComponent.bUseControllerDesiredRotation` true _charactermovement)
  (`Actor.K2_SetActorRotation` (`self.Character`) (`KismetMathLibrary.MakeRotator` 0.0 0.0 (.yaw (`Actor.K2_GetActorRotation` (`self.Character`)))) false)
  ;[1 1 1] Launch Character on exit, if needed
  (if LaunchOnExit
    (if KeepVelocity
      (`Character.LaunchCharacter` _character_3 (`KismetMathLibrary.MakeVector` 0.0 0.0 _launchvelocity) false false)
      (set `self.isClinging` false)
      (return)
      (else
        (`Character.LaunchCharacter` _character_3 (`KismetMathLibrary.MakeVector` 0.0 0.0 _launchvelocity) true true)
        (set `self.isClinging` false)
        (return)))
    (else
      (set `self.isClinging` false)
      (return))))

(fn `OnBegin`
  (params (CharacterRef :type "Character Object Reference") (LaunchSpeed :type "Float (double-precision)") (TraceDistanceRef :type "Float (double-precision)"))
  (set `self.Character` CharacterRef)
  (set `self.LaunchVelocity` LaunchSpeed)
  (set `self.TraceDistance` TraceDistanceRef)
  (bind _returnvalue (`|SpawnActorFromClass` "/Game/Clinging/Blueprints/Components/BP_BaseClingObject.BP_BaseClingObject_C" (`Actor.GetTransform` (`self.Character`)) "Undefined" "OverrideRootScale" null false false "NewEnumerator0" "NewEnumerator0" false null))
  (`Actor.SetActorHiddenInGame` _returnvalue true)
  (`PrimitiveComponent.SetCollisionResponseToAllChannels` (`/Game/Clinging/Blueprints/Components/BP_BaseClingObject.Capsule` _returnvalue) "ECR_Ignore")
  (bind _output_get (set `self.OriginalObject` _returnvalue))
  (set `self.ClingObject` _output_get))

(fn `TickFunction`
  (params (`Interpolate?` :type Boolean) (InterpSpeed :type "Float (double-precision)") (Forward :type "Float (double-precision)") (Right :type "Float (double-precision)"))
  ;[1 1 1] Only Run if Clinging is true
  (if (`self.isClinging`)
    (`self.ClingRotation(Climb)` `Interpolate?` InterpSpeed)
    (`self.GetAdjacentObject` Forward Right)
    ;[0.2601 1 0.3249] Launch up when close enough to flat edge
    (`self.GetObjectSurface`)
    (`self.IsOnGround`))
  (return))