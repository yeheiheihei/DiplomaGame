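; Cinematic figure actor whose skeletal mesh (Rope) starts invisible and fades in through a material Opacity parameter when PlayAnim runs.
; With IsTriggerWork set, MyChar must stay inside the sphere beyond SeeeTime to trigger it through a DoOnce.
; It either holds for ShowTime (HaveSpline) or plays Anim once, freezing just before the end.
; A second timeline then fades it out and re-arms the DoOnce.
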(event `self.ReceiveBeginPlay`
  (`self.SetOpacity` 0.0)
  (if (not (`self.IsTriggerWork?`))
    (`ActorComponent.K2_DestroyComponent` (`self.Sphere`))))

(event `PlayAnim`
  (bind _anim (`self.Anim`))
  (bind _rope (`self.Rope`))
  (`|ExecutionSequence`
    (:`then_0`
      ;[1 0.05535 0.8201] 渐隐
      (bind (_direction _alpha) (`Timeline|Timeline_0` :!via `PlayFromStart`)
        (:`Update`
          (`self.SetOpacity` _alpha))))
    (:`then_1`
      (`SkeletalMeshComponent.SetPlayRate` (`self.Rope`) (`self.PlayRate`))
      (if (`self.HaveSpline？`)
        (`KismetSystemLibrary.Delay` (`self.ShowTime`))
        ;[1 0.156 0.1759 1 37] 渐隐
        (bind (_direction_2 _alpha_2 _opacity) (`Timeline|Timeline_1` :!via `PlayFromStart` :!label _label)
          (:`Update`
            (`self.SetOpacity` _opacity))
          (:`Finished`
            (goto _label_2 :!via `Reset`)))
        (else
          (`SkeletalMeshComponent.PlayAnimation` _rope _anim false)
          (`KismetSystemLibrary.Delay` (- (`AnimSequenceBase.SequenceLength` _anim) 0.5))
          (`SkeletalMeshComponent.SetPlayRate` _rope 0.0)
          (goto _label :!via `PlayFromStart`))))))

(event `self.ReceiveTick`
  (params (DeltaSeconds :type "Float (single-precision)"))
  (if (`self.IsIn`)
    (bind _output_get (set `self.Timer` (+ (`self.Timer`) DeltaSeconds)))
    (`/Engine/EditorBlueprintResources/StandardMacros.CompareFloat` _output_get (`self.SeeeTime`)
      (:`>`
        (set `self.IsIn` false)
        (`/Engine/EditorBlueprintResources/StandardMacros.DoOnce` false :!label _label_2
          (:`Completed`
            (`self.PlayAnim`)))))))

(event `self.Sphere.OnComponentBeginOverlap`
  (params (OverlappedComponent :type "PrimitiveComponent Object Reference") (OtherActor :type "Actor Object Reference") (OtherComp :type "PrimitiveComponent Object Reference") (OtherBodyIndex :type Integer) (bFromSweep :type Boolean) (SweepResult :type "HitResult Structure (by ref)"))
  (cast `/Game/Blueprints/Hero/MyChar` OtherActor)
  (set `self.IsIn` true))

(event `self.Sphere.OnComponentEndOverlap`
  (params (OverlappedComponent :type "PrimitiveComponent Object Reference") (OtherActor :type "Actor Object Reference") (OtherComp :type "PrimitiveComponent Object Reference") (OtherBodyIndex :type Integer))
  (cast `/Game/Blueprints/Hero/MyChar` OtherActor)
  (set `self.IsIn` false)
  (set `self.Timer` 0.0))

(fn `SetOpacity`
  (params (Opacity :type "Float (double-precision)"))
  (`MeshComponent.SetScalarParameterValueOnMaterials` (`self.Rope`) "Opacity" Opacity))

(fn `UserConstructionScript`)