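; GameManager blueprint that finds the nearest findable point in its Points array to a given position.
; GetLinerPoint and GetLinerPoints drop entries with CanbeFound off while looping, then scan the rest for the shortest distance.
; Both draw a debug trace to the winner, but only GetLinerPoints returns its location.
; The event's wind source lookup goes unused, and a collapsed variant of the search never runs.
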(event `self.ReceiveBeginPlay`
  ;[1 1 1] 之后修改
  (set `self.DistanceIndex` 0))

(event `GetLinerPoint`
  (params (TriggerPos :type "Vector Structure"))
  (for (_array_element _array_index) (`self.Points`)
    (if (not (`/Game/Blueprints/Misc/MamiVal.CanbeFound` _array_element))
      (`KismetArrayLibrary.Array_Remove` (`self.Points`) _array_index)))
  (set `self.DistanceIndex` 0)
  (set `self.Distance` (`self.VectorLength` (`/Game/Blueprints/Misc/MamiVal.ReturnDir` (`|GetArrayItem` (`self.Points`) (`self.DistanceIndex`))) TriggerPos))
  (for (_array_element_2 _array_index_2) (`self.Points`)
    (bind _length (`self.VectorLength` (`/Game/Blueprints/Misc/MamiVal.ReturnDir` _array_element_2) TriggerPos))
    (if (< _length (`self.Distance`))
      (set `self.Distance` _length)
      (set `self.DistanceIndex` _array_index_2)))
  (`KismetSystemLibrary.LineTraceSingle` :`Start` (+ TriggerPos (0.0 0.0 100.0)) :`End` (+ (`self.K2_GetActorLocation` (`|GetArrayItem` (`self.Points`) (`self.DistanceIndex`))) (0.0 0.0 100.0)) :`TraceChannel` "TraceTypeQuery1" :`DrawDebugType` "ForDuration")
  (bind _outactors (`GameplayStatics.GetAllActorsOfClass` "/Script/Engine.WindDirectionalSource")))

(fn `GetLinerPoints`
  (params (Pos :type "Vector Structure"))
  (returns (TargetPos :type "Vector Structure"))
  (bind _returnvalue (`self.K2_GetActorLocation` (`|GetArrayItem` (`self.Points`) (`self.DistanceIndex`))))
  (for (_array_element _array_index) (`self.Points`)
    (if (not (`/Game/Blueprints/Misc/MamiVal.CanbeFound` _array_element))
      (`KismetArrayLibrary.Array_Remove` (`self.Points`) _array_index)))
  (set `self.DistanceIndex` 0)
  (set `self.Distance` (`self.VectorLength` (`/Game/Blueprints/Misc/MamiVal.ReturnDir` (`|GetArrayItem` (`self.Points`) (`self.DistanceIndex`))) Pos))
  (for (_array_element_2 _array_index_2) (`self.Points`)
    (bind _length (`self.VectorLength` (`/Game/Blueprints/Misc/MamiVal.ReturnDir` _array_element_2) Pos))
    (if (< _length (`self.Distance`))
      (set `self.Distance` _length)
      (set `self.DistanceIndex` _array_index_2)))
  (`KismetSystemLibrary.LineTraceSingle` :`Start` (+ Pos (0.0 0.0 100.0)) :`End` (+ _returnvalue (0.0 0.0 100.0)) :`TraceChannel` "TraceTypeQuery1" :`DrawDebugType` "ForDuration")
  (return _returnvalue))

(fn `UserConstructionScript`)

(fn `VectorLength`
  (params (pos :type "Vector Structure") (TriggerPos :type "Vector Structure"))
  (returns (length :type "Float (double-precision)"))
  (bind _returnvalue (`KismetMathLibrary.VSize` (- pos TriggerPos)))
  (`KismetSystemLibrary.PrintString` (`KismetStringLibrary.Concat_StrStr` "长度" (`KismetStringLibrary.Conv_DoubleToString` _returnvalue)))
  (return _returnvalue))