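; OldPeople is an elderly NPC that walks from its starting spot to one of a set of target points.
; It records its location on BeginPlay as its home position.
; MoveTo snaps it back to that position without a sweep, then has its AI controller path to the target point at the given index.
; Nothing in this Blueprint calls MoveTo, and a leftover SimpleMoveToLocation node never runs.
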(event `self.ReceiveBeginPlay`
  (set `self.OriPos` (`self.K2_GetActorLocation`)))

(fn `MoveTo`
  (params (index :type Integer))
  (`self.K2_SetActorLocation` (`self.OriPos`))
  (`AIController.MoveToLocation` (`AIBlueprintHelperLibrary.GetAIController` self) (`self.K2_GetActorLocation` (`|GetArrayItem` (`self.targetpoints`) index)) -1.0 true true false true null true))

(fn `UserConstructionScript`)