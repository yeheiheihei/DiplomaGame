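; SaveGameManager restores a level checkpoint when ReadGame is called with a stage enum (giant tree, multi-layer trees, lotus leaf, Boss).
; The enum selects a SaveArray entry, whose valid AICharacter actors get ChangeBack, while AIBoss entries are cast but left untouched.
; It then moves the player to the entry's PlayerPos actor transform, clears the SeeEnemy UI state and calls the player's ChangeBack.
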(event `ReadGame`
  (params (ChangeEnum :type "/Game/Blueprints/OtherChar/SaveEnum Enum" :default "NewEnumerator0"))
  (bind _returnvalue (`GameplayStatics.GetPlayerCharacter` 0))
  (bind (_output_playerpos _output_ai) (break `/Game/Blueprints/OtherChar/SaveStruct` (`|GetArrayItem` (`self.SaveArray`) (`self.Index`))))
  (switch `/Game/Blueprints/OtherChar/SaveEnum` ChangeEnum
    (:`NewEnumerator0`
      (set `self.Index` 0))
    (:`NewEnumerator1`
      (set `self.Index` 1))
    (:`NewEnumerator2`
      (set `self.Index` 2))
    (:`NewEnumerator3`
      (set `self.Index` 3)))
  (for _array_element _output_ai
    (`/Engine/EditorBlueprintResources/StandardMacros.IsValid` _array_element
      (:`Is Valid`
        (bind _asaicharacter (cast `/Game/AI/AICharacter` _array_element)
          (:`then`
            (`/Game/AI/AICharacter.ChangeBack` _asaicharacter))
          (:`CastFailed`
            (cast `/Game/AI/BIgBoss/AIBoss` _array_element))))))
  ;[1 1 1] 音乐
  (`self.K2_SetActorTransform` _returnvalue (`self.GetTransform` _output_playerpos) false false)
  (bind _asmy_char (cast `/Game/Blueprints/Hero/MyChar` _returnvalue))
  (`/Game/UI/Player.SeeEnemy` (`/Game/Blueprints/Hero/MyChar.PlayerUI` _asmy_char) false)
  (`/Game/Blueprints/Hero/MyChar.ChangeBack` _asmy_char))

(fn `UserConstructionScript`)