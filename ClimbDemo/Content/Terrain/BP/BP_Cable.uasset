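; Cable actor that swings side to side with a plane riding along on it, animated every frame.
; Tick drives the CableComponent's force along X with a sine of game time, producing a steady oscillation.
; The plane is then moved to the world location of one fixed cable particle, so it follows the simulated motion without rotating.
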(event `self.ReceiveTick`
  (params (DeltaSeconds :type "Float (single-precision)"))
  (set `CableComponent.CableForce` (`KismetMathLibrary.MakeVector` (* (`KismetMathLibrary.Sin` (* (`KismetSystemLibrary.GetGameTimeInSeconds`) 5.0)) 2000.0)) (`self.CableComponent`))
  (`SceneComponent.K2_SetWorldLocation` (`self.Plane`) (`|GetArrayItem` (`CableComponent.GetCableParticleLocations` (`self.CableComponent`)) 6) false false))

(fn `UserConstructionScript`)